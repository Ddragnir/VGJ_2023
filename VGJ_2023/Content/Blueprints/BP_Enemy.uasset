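; BP_Enemy is an enemy character that chases the player by issuing AIMoveTo every Tick.
; Damage spawns a damage actor and reveals a widget life bar, hidden at start and scaled for 100 life.
; At zero life it drops a BP_Experience and destroys itself; Reset destroys it without a drop.
; ApplySpeedPercent temporarily scales walk speed, using a retriggerable delay to restore it.
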(event Custom|Reset
  (Actor|DestroyActor))

(event Custom|EventConstruct)

(event Custom|SetLifeBarVisibility
  (params (bNewVisibility :type Boolean))
  (Rendering|SetVisibility (Variables|Default|GetLifeBar) bNewVisibility false))

(event Custom|SetLifeBarValue
  (params (LifeValue :type Float%20%28double-precision%29))
  (Default|SetLifeBarValue (Variables|Default|GetLifeBarWidget) (/ LifeValue 1e+02)))

(event EventBeginPlay
  (bind _asbp_player (Utilities|Casting|CastToBP_Player (Game|GetPlayerCharacter 0)))
  (Variables|Default|SetPlayer _asbp_player)
  (Variables|/Script/Engine.CharacterMovementComponent|SetMaxWalkSpeed (Variables|Character|GetCharacterMovement) (Variables|Default|GetEnemySpeed))
  (bind _aswg_life_bar (Utilities|Casting|CastToWG_LifeBar (UserInterface|GetWidget (Variables|Default|GetLifeBar))))
  (Variables|Default|SetLifeBarWidget _aswg_life_bar)
  (CallFunction|SetLifeBarValue 1e+02)
  (CallFunction|SetLifeBarVisibility false))

(event EventTick
  (params (DeltaSeconds :type Float%20%28single-precision%29))
  (AI|AIMoveTo self "0, 0, 0" (Variables|Default|GetPlayer) 1e+02 false))

(event EventApplySpeedPercent
  (params (Percent :type Float%20%28double-precision%29) (Duration :type Float%20%28double-precision%29))
  (Variables|/Script/Engine.CharacterMovementComponent|SetMaxWalkSpeed (Variables|Character|GetCharacterMovement) (* (/ Percent 1e+02) (Variables|Default|GetEnemySpeed)))
  (Utilities|FlowControl|RetriggerableDelay Duration)
  (Variables|/Script/Engine.CharacterMovementComponent|SetMaxWalkSpeed (Variables|Character|GetCharacterMovement) (Variables|Default|GetEnemySpeed)))

(event EventApplyDamage
  (params (Damage :type Float%20%28double-precision%29) (FromPlayer? :type Boolean))
  (bind _output_get (Variables|Default|SetEnemyLife (- (Variables|Default|GetEnemyLife) Damage)))
  (Game|SpawnActorfromClass "/Game/Blueprints/BP_DamageActor.BP_DamageActor_C" (Transformation|GetActorTransform) "Undefined" "MultiplyWithRoot" 0 (Math|Float|Truncate Damage) 0)
  (CallFunction|SetLifeBarVisibility true)
  (CallFunction|SetLifeBarValue (Variables|Default|GetEnemyLife))
  (if (<= _output_get 0.0)
    (Game|SpawnActorfromClass "/Game/Blueprints/BP_Experience.BP_Experience_C" (Math|Transform|MakeTransform (Transformation|GetActorLocation) (Transformation|GetActorRotation)) "Undefined" "MultiplyWithRoot" 0 0)
    (Actor|DestroyActor)))

(fn ConstructionScript
  (CallFunction|EventConstruct))