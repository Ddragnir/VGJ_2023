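; BP_CameraMenu is the menu camera actor that shows the main menu at game start and again through its FromGameOver event.
; It creates or re-shows the WG_Menu widget with the cursor visible and fills it with money and each upgrade's price and count read from BP_Player.
; StartButton hides the menu, blends the view to the player over a short delay, then possesses it.
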(event Custom|ShowMenuWidget
  (params (InVisibility :type ESlateVisibility%20Enum :default "Visible"))
  (Widget|SetVisibility (Variables|Default|GetMenu) InVisibility))

(event Custom|StartButton
  (bind _returnvalue (Game|GetPlayerController 0))
  (bind _playerref (Variables|Default|GetPlayerRef))
  (CallFunction|ShowMenuWidget "Hidden")
  (Game|Player|SetViewTargetwithBlend _returnvalue _playerref 1.0 "VTBlend_Linear" 0.0 false)
  (Utilities|FlowControl|Delay 1.0)
  (Pawn|Possess _returnvalue _playerref)
  (Default|Possess _playerref))

(event Custom|FromGameOver
  (bind _outactors (Actor|GetAllActorsOfClass "/Game/Blueprints/BP_Player.BP_Player_C"))
  (Variables|Default|SetPlayerRef (Utilities|Array|Get(acopy) _outactors))
  (Variables|/Script/Engine.PlayerController|SetbShowMouseCursor (Game|GetPlayerController 0) true)
  (bind _returnvalue (UserInterface|CreateWidget "/Game/Blueprints/WG_Menu.WG_Menu_C" (Game|GetPlayerController 0)))
  (Utilities|IsValid (Variables|Default|GetMenu)
    (:Is%20Valid
      (CallFunction|ShowMenuWidget "Visible"))
    (:Is%20Not%20Valid
      (bind _output_get (Variables|Default|SetMenu _returnvalue))
      (UserInterface|Viewport|AddtoViewport _output_get 0)))
  (Default|SetupMoney (Variables|Default|GetMenu) (Utilities|Text|ToText(Integer) (Variables|/Game/Blueprints/BP_Player.BP_Player_C|GetMoney (Variables|Default|GetPlayerRef))))
  (Default|SetUpPioche (Variables|Default|GetMenu) (Utilities|Text|ToText(Integer) (Variables|/Game/Blueprints/BP_Player.BP_Player_C|GetPiocherPrice (Variables|Default|GetPlayerRef))) (Utilities|Text|ToText(Integer) (Variables|/Game/Blueprints/BP_Player.BP_Player_C|GetPiocherCount (Variables|Default|GetPlayerRef))))
  (Default|SetupAugmentez (Variables|Default|GetMenu) (Utilities|Text|ToText(Integer) (Variables|/Game/Blueprints/BP_Player.BP_Player_C|GetAugmenterExpPrice (Variables|Default|GetPlayerRef))) (Utilities|Text|ToText(Integer) (Variables|/Game/Blueprints/BP_Player.BP_Player_C|GetAugmenterExpCount (Variables|Default|GetPlayerRef))))
  (Default|SetupRelancez (Variables|Default|GetMenu) (Utilities|Text|ToText(Integer) (Variables|/Game/Blueprints/BP_Player.BP_Player_C|GetRelancerPrice (Variables|Default|GetPlayerRef))) (Utilities|Text|ToText(Integer) (Variables|/Game/Blueprints/BP_Player.BP_Player_C|GetRelancerCount (Variables|Default|GetPlayerRef))))
  (Default|SetupChoisissez (Variables|Default|GetMenu) (Utilities|Text|ToText(Integer) (Variables|/Game/Blueprints/BP_Player.BP_Player_C|GetChoosePlusPrice (Variables|Default|GetPlayerRef))) (Utilities|Text|ToText(Integer) (Variables|/Game/Blueprints/BP_Player.BP_Player_C|GetChoosePlusCount (Variables|Default|GetPlayerRef)))))

(event EventBeginPlay
  (bind _outactors (Actor|GetAllActorsOfClass "/Game/Blueprints/BP_Player.BP_Player_C"))
  (Variables|Default|SetPlayerRef (Utilities|Array|Get(acopy) _outactors))
  (Variables|/Script/Engine.PlayerController|SetbShowMouseCursor (Game|GetPlayerController 0) true)
  (bind _returnvalue (UserInterface|CreateWidget "/Game/Blueprints/WG_Menu.WG_Menu_C" (Game|GetPlayerController 0)))
  (Utilities|IsValid (Variables|Default|GetMenu)
    (:Is%20Valid
      (CallFunction|ShowMenuWidget "Visible"))
    (:Is%20Not%20Valid
      (bind _output_get (Variables|Default|SetMenu _returnvalue))
      (UserInterface|Viewport|AddtoViewport _output_get 0)))
  (Default|SetupMoney (Variables|Default|GetMenu) (Utilities|Text|ToText(Integer) (Variables|/Game/Blueprints/BP_Player.BP_Player_C|GetMoney (Variables|Default|GetPlayerRef))))
  (Default|SetUpPioche (Variables|Default|GetMenu) (Utilities|Text|ToText(Integer) (Variables|/Game/Blueprints/BP_Player.BP_Player_C|GetPiocherPrice (Variables|Default|GetPlayerRef))) (Utilities|Text|ToText(Integer) (Variables|/Game/Blueprints/BP_Player.BP_Player_C|GetPiocherCount (Variables|Default|GetPlayerRef))))
  (Default|SetupAugmentez (Variables|Default|GetMenu) (Utilities|Text|ToText(Integer) (Variables|/Game/Blueprints/BP_Player.BP_Player_C|GetAugmenterExpPrice (Variables|Default|GetPlayerRef))) (Utilities|Text|ToText(Integer) (Variables|/Game/Blueprints/BP_Player.BP_Player_C|GetAugmenterExpCount (Variables|Default|GetPlayerRef))))
  (Default|SetupRelancez (Variables|Default|GetMenu) (Utilities|Text|ToText(Integer) (Variables|/Game/Blueprints/BP_Player.BP_Player_C|GetRelancerPrice (Variables|Default|GetPlayerRef))) (Utilities|Text|ToText(Integer) (Variables|/Game/Blueprints/BP_Player.BP_Player_C|GetRelancerCount (Variables|Default|GetPlayerRef))))
  (Default|SetupChoisissez (Variables|Default|GetMenu) (Utilities|Text|ToText(Integer) (Variables|/Game/Blueprints/BP_Player.BP_Player_C|GetChoosePlusPrice (Variables|Default|GetPlayerRef))) (Utilities|Text|ToText(Integer) (Variables|/Game/Blueprints/BP_Player.BP_Player_C|GetChoosePlusCount (Variables|Default|GetPlayerRef)))))

(fn ConstructionScript)