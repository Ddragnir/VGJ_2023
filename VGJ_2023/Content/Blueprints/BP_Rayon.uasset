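; BP_Rayon is a chaining beam that jumps between actors, damaging one per hop.
; CallRayon sphere-traces around itself, selects the last unique hit, then line-traces toward it, so a different actor in the way takes the damage instead.
; Each hop plays beam and impact Niagara effects and sounds.
; While Count remains, it recursively spawns another BP_Rayon at the trace end, passing along a growing ignore list.
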(event Custom|CallRayon
  (params (ActorsToIgnore :type Array%20of%20Actor%20Object%20References) (Count :type Integer))
  (bind _returnvalue (Transformation|GetActorLocation))
  (bind _returnvalue_2 (Transformation|GetActorLocation))
  (bind _hitactors (Variables|Default|GetHitActors))
  (bind _output_get (Variables|Default|SetActors%20to%20Ignore ActorsToIgnore))
  (bind _result (Math|Integer|DecrementInt Count)
    (:%20%20
      (Variables|Default|SetCount _result)
      (bind _outhits (Collision|MultiSphereTraceByChannel _returnvalue _returnvalue (Variables|Default|GetRayonArea) "TraceTypeQuery3" false _output_get "None" true "(R=1.000000,G=0.000000,B=0.000000,A=1.000000)" "(R=0.000000,G=1.000000,B=0.000000,A=1.000000)" 1.0))
      (for _array_element _outhits
        (Utilities|Array|AddUnique (Variables|Default|GetHitActors) (.HitActor (Collision|BreakHitResult _array_element))))
      (bind _output_get_2 (Variables|Default|SetSelectedActor (Utilities|Array|Get(acopy) _hitactors (- (Utilities|Array|Length _hitactors) 1))))
      (Utilities|IsValid _output_get_2
        (:Is%20Valid
          (bind _outhit (Collision|LineTraceByChannel _returnvalue_2 (Transformation|GetActorLocation _output_get_2) "TraceTypeQuery3" false 0 "None" true "(R=1.000000,G=0.000000,B=0.000000,A=1.000000)" "(R=0.000000,G=1.000000,B=0.000000,A=1.000000)" 1.0))
          (bind _returnvalue_3 (Niagara|SpawnSystematLocation "/Game/VFX/NS_Beam.NS_Beam" _returnvalue_2))
          (Audio|SpawnSoundatLocation "/Game/AUDIO/SFX/SND_Beam_Cue.SND_Beam_Cue" _returnvalue_2 "0, 0, 0" 1.0 1.0 0.0 0 0)
          (Niagara|SetNiagaraVariable(Vector3) _returnvalue_3 "LaserEnd" (.TraceEnd (Collision|BreakHitResult _outhit)))
          (Niagara|SpawnSystematLocation "/Game/VFX/NS_BeamHit.NS_BeamHit" (.TraceEnd (Collision|BreakHitResult _outhit)))
          (Audio|SpawnSoundatLocation "/Game/AUDIO/SFX/SND_BeamHit_Cue.SND_BeamHit_Cue" (.TraceEnd (Collision|BreakHitResult _outhit)) "0, 0, 0" 1.0 1.0 0.0 0 0)
          (Class|ITInterraction|ApplyDamage(Message) (select (== (.HitActor (Collision|BreakHitResult _outhit)) (Variables|Default|GetSelectedActor)) (Variables|Default|GetSelectedActor) (.HitActor (Collision|BreakHitResult _outhit))) (Variables|Default|GetRayonDamage) "NewEnumerator0")
          (Utilities|IsValid (select (== (.HitActor (Collision|BreakHitResult _outhit)) (Variables|Default|GetSelectedActor)) (Variables|Default|GetSelectedActor) (.HitActor (Collision|BreakHitResult _outhit)))
            (:Is%20Valid
              (Utilities|Array|AddUnique (Variables|Default|GetActors%20to%20Ignore) (select (== (.HitActor (Collision|BreakHitResult _outhit)) (Variables|Default|GetSelectedActor)) (Variables|Default|GetSelectedActor) (.HitActor (Collision|BreakHitResult _outhit)))))
            (:Is%20Not%20Valid
              _))
          (if (> (Variables|Default|GetCount) 0)
            (bind _returnvalue_4 (Game|SpawnActorfromClass "BP_Rayon_C" (Math|Transform|MakeTransform (.TraceEnd (Collision|BreakHitResult _outhit)) "0, 0, 0" "1.000000,1.000000,1.000000") "Undefined" "MultiplyWithRoot" 0 (Variables|Default|GetRayonArea) (Variables|Default|GetRayonDamage) 0))
            (CallFunction|CallRayon _returnvalue_4 (Variables|Default|GetActors%20to%20Ignore) (Variables|Default|GetCount))))))))

(fn ConstructionScript)