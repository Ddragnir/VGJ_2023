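; BP_RockFall is a self-running falling rock effect that starts on BeginPlay.
; It gives the rock mesh a slight random yaw, then a timeline lerps its world Z from 3000 down to zero, keeping X and Y.
; On finish it spawns a Niagara explosion at the fall effect's location, destroys the rock and mark components, and deactivates the fall effect.
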(event EventBeginPlay
  (bind _rock03 (Variables|Default|Getrock03))
  (bind _returnvalue (Transformation|GetWorldLocation _rock03))
  (Transformation|SetWorldRotation (Variables|Default|Getrock03) (Math|Rotator|MakeRotator 0.0 0.0 (Math|Random|RandomFloatinRange 0.0 1.0)) false false)
  (bind _fall (Timeline|RockFall PlayFromStart)
    (:Update
      (Transformation|SetWorldLocation _rock03 (Math|Vector|MakeVector (.x _returnvalue) (.y _returnvalue) (Math|Float|Lerp 3e+03 0.0 _fall)) false false))
    (:Finished
      (Niagara|SpawnSystematLocation "/Game/VFX/NS_RockExplosion.NS_RockExplosion" (Transformation|GetWorldLocation (Variables|Default|GetNS_RockFall)))
      (Components|DestroyComponent (Variables|Default|Getrock03))
      (Components|Activation|Deactivate (Variables|Default|GetNS_RockFall))
      (Components|DestroyComponent (Variables|Default|GetNS_RockMark)))))

(event Collision|EventActorBeginOverlap
  (params (OtherActor :type Actor%20Object%20Reference)))

(event EventTick
  (params (DeltaSeconds :type Float%20%28single-precision%29)))

(fn ConstructionScript)