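; Projectile actor that damages enemies on overlap when it is flagged as fired by the player.
; The construction script calls a construct event that sets the movement component's initial and max speed from a projectile speed variable.
; Sphere overlaps cast to BP_Enemy, send it a damage message with the projectile's damage, then destroy the projectile.
; Projectiles not from the player have no overlap response here.
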(event OnComponentBeginOverlap(Sphere)
  (params (OverlappedComponent :type Primitive%20Component%20Object%20Reference) (OtherActor :type Actor%20Object%20Reference) (OtherComp :type Primitive%20Component%20Object%20Reference) (OtherBodyIndex :type Integer) (bFromSweep :type Boolean) (SweepResult :type Hit%20Result%20Structure%20%28by%20ref%29))
  (if (Variables|Default|GetFromPlayer)
    (bind _asbp_enemy (Utilities|Casting|CastToBP_Enemy OtherActor))
    (Class|ITInterraction|ApplyDamage(Message) _asbp_enemy (Variables|Default|GetProjectileDamage) (Variables|Default|GetFromPlayer))
    (Actor|DestroyActor)))

(event Custom|EventConstruct
  (bind _projectilemovement (Variables|Default|GetProjectileMovement))
  (bind _output_get (Variables|/Script/Engine.ProjectileMovementComponent|SetInitialSpeed _projectilemovement (Variables|Default|GetProjectileSpeed)))
  (Variables|/Script/Engine.ProjectileMovementComponent|SetMaxSpeed _projectilemovement _output_get))

(fn ConstructionScript
  (CallFunction|EventConstruct))