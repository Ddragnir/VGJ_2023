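; Projectile actor that flies a sphere along an arcing spline to a target location on behalf of an Investigator.
; Setup faces the actor at the target, moves the spline's end there, and reshapes two middle points into an arc whose world height scales with spline length.
; A timeline drives the sphere along the spline, then calls BackUpBatProjectile on the Investigator, if valid, and destroys the actor.
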(event Custom|SetupParaboleProjectile
  (params (EndLocation :type Vector) (Investigator :type BP%20Enemy%20Object%20Reference))
  (bind _spline (Variables|Default|GetSpline))
  (bind _spline_2 (Variables|Default|GetSpline))
  (bind _spline_3 (Variables|Default|GetSpline))
  (bind _returnvalue (Spline|GetLocationatSplinePoint _spline_2 2 "World"))
  (bind _returnvalue_2 (Spline|GetSplineLength _spline))
  (bind _returnvalue_3 (Spline|GetLocationatSplinePoint _spline_3 1 "World"))
  (bind _output_get (Variables|Default|SetEnd%20Location EndLocation))
  (Variables|Default|SetInvestigator Investigator)
  (Transformation|SetActorRotation (Math|Rotator|FindLookatRotation (Transformation|GetActorLocation) _output_get))
  (Spline|SetLocationatSplinePoint (Variables|Default|GetSpline) 3 (Variables|Default|GetEnd%20Location) "World" true)
  (Variables|Default|SetNewVar _returnvalue_2)
  (Spline|SetLocationatSplinePoint _spline 1 (Math|Vector|MakeVector (.x (Spline|GetLocationatDistanceAlongSpline _spline (* (Variables|Default|GetNewVar) 0.3) "Local")) (.y (Spline|GetLocationatDistanceAlongSpline _spline (* (Variables|Default|GetNewVar) 0.3) "Local")) 0.0) "Local" true)
  (Variables|Default|SetNewVar _returnvalue_2)
  (Spline|SetLocationatSplinePoint _spline 2 (Math|Vector|MakeVector (.x (Spline|GetLocationatDistanceAlongSpline _spline (* (Variables|Default|GetNewVar) 0.7) "Local")) (.y (Spline|GetLocationatDistanceAlongSpline _spline (* (Variables|Default|GetNewVar) 0.7) "Local")) 0.0) "Local" true)
  (bind _output_get_2 (Variables|Default|SetNewVar _returnvalue_2))
  (Spline|SetLocationatSplinePoint _spline_3 1 (Math|Vector|MakeVector (.x _returnvalue_3) (.y _returnvalue_3) (/ _output_get_2 1.5)) "World" true)
  (Spline|SetLocationatSplinePoint _spline_2 2 (Math|Vector|MakeVector (.x _returnvalue) (.y _returnvalue) (/ _output_get_2 1.5)) "World" true)
  (CallFunction|MoveAlongSpline))

(event Custom|MoveAlongSpline
  (bind _spline (Variables|Default|GetSpline))
  (bind _investigator (Variables|Default|GetInvestigator))
  (bind _alpha (Timeline|TM_MoveAlongSpline PlayFromStart)
    (:Update
      (Transformation|SetWorldTransform (Variables|Default|GetSphere) (Math|Transform|MakeTransform (Spline|GetLocationatDistanceAlongSpline _spline (Math|Float|Lerp 0.0 (Spline|GetSplineLength (Variables|Default|GetSpline)) _alpha) "World") (Spline|GetRotationatDistanceAlongSpline _spline (Math|Float|Lerp 0.0 (Spline|GetSplineLength (Variables|Default|GetSpline)) _alpha) "World") "1.000000,1.000000,1.000000") false false))
    (:Finished
      (Utilities|IsValid _investigator
        (:Is%20Valid
          (Default|BackUpBatProjectile _investigator))
        (:Is%20Not%20Valid
          _))
      (Actor|DestroyActor))))

(fn ConstructionScript)