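; BP_IceDome is a one-shot area effect actor that applies a timed speed-percent change to actors around it.
; On BeginPlay it runs a zero-length multi sphere trace at its own location, using the dome area as radius.
; Each hit actor receives an ApplySpeedPercent message with the dome's percent and duration.
; DestroyActor sits inside the hit loop, so the dome removes itself only when something is hit.
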(event Custom|CallIceDome
  (bind _returnvalue (Transformation|GetActorLocation))
  (bind _outhits (Collision|MultiSphereTraceByChannel _returnvalue _returnvalue (Variables|Default|GetIceDomeArea) "TraceTypeQuery3" false 0 "None" true "(R=1.000000,G=0.000000,B=0.000000,A=1.000000)" "(R=0.000000,G=1.000000,B=0.000000,A=1.000000)" 1.0))
  (for _array_element _outhits
    (Class|ITInterraction|ApplySpeedPercent(Message) (.HitActor (Collision|BreakHitResult _array_element)) (Variables|Default|GetIceDomePercent) (Variables|Default|GetIceDomeDuration))
    (Actor|DestroyActor)))

(event EventBeginPlay
  (CallFunction|CallIceDome))

(fn ConstructionScript)