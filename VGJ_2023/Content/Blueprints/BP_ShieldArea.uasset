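; BP_ShieldArea is an actor that performs a one-shot area damage burst, the shield explosion, at its location when play begins.
; BeginPlay calls CallShield, which spawns the NS_ShieldExplosion Niagara system and sets its two size parameters from variables.
; A zero-length multi-sphere trace of ShieldArea radius then sends an ApplyDamage message with ShieldDammage to each hit actor.
; CallStorm and the construction script are empty.
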(event Custom|CallShield
  (bind _returnvalue (Transformation|GetActorLocation))
  (bind _returnvalue_2 (Niagara|SpawnSystematLocation "/Game/VFX/NS_ShieldExplosion.NS_ShieldExplosion" (Transformation|GetActorLocation)))
  (Niagara|SetNiagaraVariable(Float) _returnvalue_2 "Size 1" (Variables|Default|GetSizeFX_01))
  (Niagara|SetNiagaraVariable(Float) _returnvalue_2 "Size 2" (Variables|Default|GetSizeFX_02))
  (bind _outhits (Collision|MultiSphereTraceByChannel _returnvalue _returnvalue (Variables|Default|GetShieldArea) "TraceTypeQuery3" false 0 "None" true "(R=1.000000,G=0.000000,B=0.000000,A=1.000000)" "(R=0.000000,G=1.000000,B=0.000000,A=1.000000)" 1.0))
  (for _array_element _outhits
    (Class|ITInterraction|ApplyDamage(Message) (.HitActor (Collision|BreakHitResult _array_element)) (Variables|Default|GetShieldDammage) "NewEnumerator0")))

(event EventBeginPlay
  (CallFunction|CallShield))

(fn ConstructionScript)

(fn CallStorm)