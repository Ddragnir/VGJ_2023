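; Enemy attack area actor that deals area damage and plays an explosion effect and sound chosen by enemy type.
; SetupExplosionArea stores the shape, damage and enemy parameters, then destroys the actor after a delay as a fallback.
; ExploseArea runs a sphere trace, static for circles or swept start to end otherwise, on a channel picked by damage source.
; It messages damage to each hit, spawns effects, then destroys itself.
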(event Custom|SetupExplosionArea
  (params (isCircular? :type Boolean) (FromCircleCenter? :type Boolean) (DamageType :type EN_DamageType%20Enum :default "NewEnumerator0") (Size :type Float%20%28double-precision%29) (Damage :type Float%20%28double-precision%29) (StartPoint :type Vector) (EndPoint :type Vector) (Investigator :type Actor%20Object%20Reference) (Enemy :type EN_Enemys%20Enum :default "NewEnumerator6"))
  (Variables|Default|SetIs%20Circular? isCircular?)
  (Variables|Default|SetFrom%20Circle%20Center? FromCircleCenter?)
  (Variables|Default|SetDamageFrom DamageType)
  (Variables|Default|SetEnemy Enemy)
  (Variables|Default|SetSize Size)
  (Variables|Default|SetDamage Damage)
  (Variables|Default|SetStart%20Point StartPoint)
  (Variables|Default|SetEnd%20Point EndPoint)
  (Variables|Default|SetInvestigator Investigator)
  (if (Variables|Default|GetIs%20Circular?)
    _
    (else
      _))
  ;[1 1 1] AUTO DESTROY (si plus l'ennemi)
  (Utilities|FlowControl|Delay 5.0)
  (Actor|DestroyActor))

(event Custom|ExploseArea
  (bind _returnvalue (Transformation|GetActorLocation))
  (bind _start_point (Variables|Default|GetStart%20Point))
  (bind _end_point (Variables|Default|GetEnd%20Point))
  (bind _is_circular_ (Variables|Default|GetIs%20Circular?))
  (bind _enemy (Variables|Default|GetEnemy))
  (bind _from_circle_center_ (Variables|Default|GetFrom%20Circle%20Center?))
  (bind _returnvalue_2 (select _from_circle_center_ _start_point _end_point))
  (bind _outhits (Collision|MultiSphereTraceByChannel (select _is_circular_ _returnvalue_2 (Variables|Default|GetStart%20Point)) (select _is_circular_ _returnvalue_2 (Variables|Default|GetEnd%20Point)) (Variables|Default|GetSize) (Utilities|Select :Index (Variables|Default|GetDamageFrom) :NewEnumerator0 "TraceTypeQuery3" :NewEnumerator1 "TraceTypeQuery6" :NewEnumerator2 "TraceTypeQuery7") false 0 "None" true "(R=1.000000,G=0.000000,B=0.000000,A=1.000000)" "(R=0.000000,G=1.000000,B=0.000000,A=1.000000)" 1.0))
  (for _array_element _outhits
    (Class|ITInterraction|ApplyDamage(Message) (.HitActor (Collision|BreakHitResult _array_element)) (Variables|Default|GetDamage) (Variables|Default|GetDamageFrom)))
  (Niagara|SpawnSystematLocation (Utilities|Select :Index _enemy :NewEnumerator6 0 :NewEnumerator0 0 :NewEnumerator1 "/Game/VFX/NS_BomboExplosion.NS_BomboExplosion" :NewEnumerator2 "/Game/VFX/NS_FeuFoAttack.NS_FeuFoAttack" :NewEnumerator3 "/Game/VFX/NS_BatExplosion.NS_BatExplosion" :NewEnumerator4 0 :NewEnumerator5 0) _returnvalue)
  (Audio|SpawnSoundatLocation (Utilities|Select :Index _enemy :NewEnumerator6 0 :NewEnumerator0 0 :NewEnumerator1 0 :NewEnumerator2 "/Game/AUDIO/SFX/SND_FeuFoAttack_Cue.SND_FeuFoAttack_Cue" :NewEnumerator3 "/Game/AUDIO/SFX/SND_BatExplosion_Cue.SND_BatExplosion_Cue" :NewEnumerator4 0 :NewEnumerator5 0) _returnvalue "0, 0, 0" 1.0 1.0 0.0 0 0)
  (Actor|DestroyActor))

(fn ConstructionScript)