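; BP_DamageActor is a short-lived floating damage number that pops up and flies off.
; On BeginPlay it passes its Damage value to the WG_FloatingDamage user widget in its widget component.
; It then launches its Cube component with a random upward impulse and slight sideways spread as a velocity change, so physics moves the number.
; The actor destroys itself after a one-second delay.
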(event EventBeginPlay
  (bind _aswg_floating_damage (Utilities|Casting|CastToWG_FloatingDamage (UserInterface|GetUserWidgetObject (Variables|Default|GetWidget))))
  (Default|SetDamageValue _aswg_floating_damage (Variables|Default|GetDamage))
  (Physics|AddImpulse (Variables|Default|GetCube) (Math|Vector|MakeVector (Math|Random|RandomFloatinRange -1e+02 1e+02) (Math|Random|RandomFloatinRange -1e+02 1e+02) (Math|Random|RandomFloatinRange 6e+02 8e+02)) "None" true)
  (Utilities|FlowControl|Delay 1.0)
  (Actor|DestroyActor))

(fn ConstructionScript)