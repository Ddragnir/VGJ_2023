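; Experience pickup actor that flies to the player and awards experience when its BackToPlayer event is triggered.
; From BeginPlay, the XP timeline drives the world Z of the Niagara visual.
; BackToPlayer runs once, disabling cube collision and lerping the actor toward the player's live position on a timeline with adjustable speed.
; On arrival it notifies BP_Player, spawns pickup effect and sound, then destroys itself.
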(event Custom|BackToPlayer
  (Utilities|FlowControl|DoOnce false
    (:Completed
      (bind _asbp_player (Utilities|Casting|CastToBP_Player (Game|GetPlayerCharacter 0)))
      (Variables|Default|SetPlayer _asbp_player)
      (Collision|SetCollisionEnabled (Variables|Default|GetCube) "NoCollision")
      (Components|Timeline|SetPlayRate (Variables|Default|GetTM_BackToPlayer) (Variables|Default|GetBackSpeedMultiplicator))
      (Variables|Default|SetStartLocation (Transformation|GetActorLocation))
      (bind _alpha (Timeline|TM_BackToPlayer PlayFromStart)
        (:Update
          (Transformation|SetActorLocation (Math|Vector|Lerp(Vector) (Variables|Default|GetStartLocation) (Transformation|GetActorLocation (Variables|Default|GetPlayer)) _alpha) false false))
        (:Finished
          (Default|ExperienceTaked (Variables|Default|GetPlayer))
          (Niagara|SpawnSystematLocation "/Game/VFX/NS_XPTake.NS_XPTake" (Transformation|GetWorldLocation (Variables|/Script/Engine.Character|GetCapsuleComponent (Variables|Default|GetPlayer))))
          (Audio|SpawnSound2D "/Game/AUDIO/SFX/SND_XP.SND_XP" 1.0 1.0 0.0 0)
          (Actor|DestroyActor))))))

(event EventBeginPlay
  (bind _ns_xp (Variables|Default|GetNS_XP))
  (bind _returnvalue (Transformation|GetWorldLocation _ns_xp))
  (bind _z (Timeline|XP PlayFromStart)
    (:Update
      (Transformation|SetWorldLocation _ns_xp (Math|Vector|MakeVector (.x _returnvalue) (.y _returnvalue) _z) false false))))

(fn ConstructionScript)