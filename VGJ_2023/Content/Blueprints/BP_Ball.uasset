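; BP_Ball is a player-side orb weapon that damages enemies it touches.
; On BeginPlay it offsets its Sphere component along local X by BallPlayerDistance, holding it away from the actor's origin.
; When the sphere begins overlapping a BP_Enemy, it spawns an orb-hit effect and sound at the enemy's capsule, then sends BallDamage through ApplyDamageMessage, flagged as coming from the player.
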(event OnComponentBeginOverlap(Sphere)
  (params (OverlappedComponent :type Primitive%20Component%20Object%20Reference) (OtherActor :type Actor%20Object%20Reference) (OtherComp :type Primitive%20Component%20Object%20Reference) (OtherBodyIndex :type Integer) (bFromSweep :type Boolean) (SweepResult :type Hit%20Result%20Structure%20%28by%20ref%29))
  (bind _asbp_enemy (Utilities|Casting|CastToBP_Enemy OtherActor))
  (Niagara|SpawnSystematLocation "/Game/VFX/NS_OrbHit.NS_OrbHit" (Transformation|GetWorldLocation (Variables|/Script/Engine.Character|GetCapsuleComponent _asbp_enemy)))
  (Audio|SpawnSoundatLocation "/Game/AUDIO/SFX/SND_OrbHit_Cue.SND_OrbHit_Cue" (Transformation|GetWorldLocation (Variables|/Script/Engine.Character|GetCapsuleComponent _asbp_enemy)) "0, 0, 0" 1.0 1.0 0.0 0 0)
  (Class|ITInterraction|ApplyDamage(Message) _asbp_enemy (Variables|Default|GetBallDamage) "NewEnumerator0" true))

(event EventBeginPlay
  (Transformation|SetRelativeLocation (Variables|Default|GetSphere) (Math|Vector|MakeVector (Variables|Default|GetBallPlayerDistance) 0.0 0.0) false false))

(fn ConstructionScript)