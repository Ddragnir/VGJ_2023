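; BP_WaveManager spawns BP_Enemy actors around the player on an escalating timer between StartSpawn and StopSpawn.
; Tick turns elapsed time over the saved total into a magma value, which it sends to PlayerRef and uses to shorten spawn delays and widen the random enemy-type pool.
; Spawn points are random reachable navigation points, retried until one lies far from the player and outside the forward view.
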(event Custom|StartSpawn
  (params (PlayerRef :type BP%20Player%20Object%20Reference))
  (Variables|Default|SetPlayer%20Ref PlayerRef)
  (Variables|Default|SetSavedTimer (Variables|Default|GetTotalTimer))
  (Variables|Default|SetOldSpawnDelay 0.0)
  (Variables|Default|SetDelta%20Seconds 0.0)
  (Variables|Default|SetisSpawning? true))

(event Custom|StopSpawn
  (Variables|Default|SetisSpawning? false)
  (Utilities|FlowControl|Sequence))

(event EventTick
  (params (DeltaSeconds :type Float%20%28single-precision%29))
  (bind _returnvalue (Game|Player|GetPlayerPawn 0))
  (bind _returnvalue_2 (Transformation|GetActorLocation _returnvalue))
  (if (Variables|Default|GetisSpawning?)
    (Variables|Default|SetDelta%20Seconds (+ DeltaSeconds (Variables|Default|GetDelta%20Seconds)))
    (bind _output_get (Variables|Default|SetMagmaValue (/ (Variables|Default|GetDelta%20Seconds) (Variables|Default|GetSavedTimer))))
    (Default|SetMagmaValue (Variables|Default|GetPlayer%20Ref) _output_get)
    (Variables|Default|SetSpawnDelay (Math|Float|Clamp(Float) (Math|Float|Lerp 4.0 0.3 _output_get) 1.0 4.0))
    (if (> (Variables|Default|GetDelta%20Seconds) (+ (Variables|Default|GetOldSpawnDelay) (Variables|Default|GetSpawnDelay)))
      (Variables|Default|SetOldSpawnDelay (Variables|Default|GetDelta%20Seconds))
      (bind _output_get_2 (Variables|Default|SetRandomPointNav (.RandomLocation (AI|Navigation|GetRandomReachablePointinRadius _returnvalue_2 5e+03 0 0)) :!label _label))
      (if (and (Math|Float|InRange(Float) (Math|Vector|DotProduct (Transformation|GetActorForwardVector _returnvalue) (Math|Vector|GetForwardVector (Math|Rotator|FindLookatRotation _returnvalue_2 _output_get_2))) -1.0 0.5) (> (Math|Vector|VectorLength (- _returnvalue_2 _output_get_2)) 2.2e+03))
        (if (< (Variables|Default|GetMagmaValue) 0.1)
          (Variables|Default|SetMax 0)
          (elif (< (Variables|Default|GetMagmaValue) 0.2)
            _
            (elif (< (Variables|Default|GetMagmaValue) 0.3)
              (Variables|Default|SetMax 2)
              (elif (< (Variables|Default|GetMagmaValue) 0.5)
                (Variables|Default|SetMax 3)
                (else
                  (Variables|Default|SetMax 4))))))
        (Game|SpawnActorfromClass "/Game/Blueprints/BP_Enemy.BP_Enemy_C" (Math|Transform|MakeTransform _output_get_2 "0, 0, 0" "1.000000,1.000000,1.000000") "Undefined" "MultiplyWithRoot" 0 (Utilities|Select :Index (Math|Random|RandomIntegerinRange 0 (Variables|Default|GetMax)) :Option%200 "NewEnumerator0" :Option%201 "NewEnumerator2" :Option%202 "NewEnumerator4" :Option%203 "NewEnumerator3" :Option%204 "NewEnumerator1") 0)
        (else
          (goto _label))))))

(fn ConstructionScript)